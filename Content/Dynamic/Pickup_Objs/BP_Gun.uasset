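; BP_Gun is a gun pickup that also handles its own shooting input.
; Its trigger zone sets GunPickedup on an overlapping third-person character; leaving the zone does not clear it.
; Player 0 input is enabled at BeginPlay, so Shoot checks the character's CurrentWeapon and Holding, then spawns a scaled-down BulletBP at BulletRef.
; The bullet's Z axis follows BulletRef's forward vector; several unconnected knife, tag and reset nodes never run.
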(event `self.ReceiveBeginPlay`
  (`self.EnableInput` (`GameplayStatics.GetPlayerController` 0)))

(event `InputAction|Shoot`
  (params (Key :type "Key Structure")))

(event `InputAction|Shoot`
  (params (Key :type "Key Structure"))
  (bind _bulletref (`self.BulletRef`))
  (:`Pressed`
    (bind _asbp_third_person_character (cast `/Game/Dynamic/ThirdPerson/Blueprints/BP_ThirdPersonCharacter` (`GameplayStatics.GetPlayerCharacter` 0)))
    (if (`|EnumEquality` (`/Game/Dynamic/ThirdPerson/Blueprints/BP_ThirdPersonCharacter.CurrentWeapon` _asbp_third_person_character) "NewEnumerator0")
      (if (`/Game/Dynamic/ThirdPerson/Blueprints/BP_ThirdPersonCharacter.Holding?` _asbp_third_person_character)
        (`|SpawnActorFromClass` "/Game/Dynamic/Pickup_Objs/BulletBP.BulletBP_C" (`KismetMathLibrary.MakeTransform` (`SceneComponent.K2_GetComponentLocation` _bulletref) (`KismetMathLibrary.MakeRotFromZ` (`SceneComponent.GetForwardVector` _bulletref)) (0.2 0.2 0.2)) "Undefined" "MultiplyWithRoot" null null)
        (else
          (`KismetSystemLibrary.PrintString` "No Gun"))))))

(event `/Game/Dynamic/ThirdPerson/Blueprints/BPI_Character_Info.Update Weapon Type`
  (params (EWeaponType :type "/Game/Dynamic/Pickup_Objs/WeaponsEnum Enum" :default "NewEnumerator0"))
  (set `self.weaponType` EWeaponType))

(event `self.TriggerZone.OnComponentBeginOverlap`
  (params (OverlappedComponent :type "PrimitiveComponent Object Reference") (OtherActor :type "Actor Object Reference") (OtherComp :type "PrimitiveComponent Object Reference") (OtherBodyIndex :type Integer) (bFromSweep :type Boolean) (SweepResult :type "HitResult Structure (by ref)"))
  (bind _asbp_third_person_character (cast `/Game/Dynamic/ThirdPerson/Blueprints/BP_ThirdPersonCharacter` OtherActor))
  (set `/Game/Dynamic/ThirdPerson/Blueprints/BP_ThirdPersonCharacter.GunPickedup?` true _asbp_third_person_character))

(event `self.TriggerZone.OnComponentEndOverlap`
  (params (OverlappedComponent :type "PrimitiveComponent Object Reference") (OtherActor :type "Actor Object Reference") (OtherComp :type "PrimitiveComponent Object Reference") (OtherBodyIndex :type Integer)))

(fn `Essential Values`
  (returns (`Aiming Rotation` :type "Rotator Structure"))
  (return))

(fn `UserConstructionScript`)