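; Enemy spawner actor that spawns queued enemy classes at its own transform and reports defeated enemies to BP_GameMode.
; AddEnemyToQueue appends a class and spawns the queue head immediately if no BP_AI overlaps its Sphere.
; A looping BeginPlay timer also pops the queue, without that overlap check.
; Each spawn binds OnDestroyed for defeat reporting; older random-point, count-capped spawning remains as unused code.
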(event `OnEnemyDeafeated`
  (params (DestroyedActor :type "Actor Object Reference"))
  (bind _asbp_game_mode (cast `/Game/Dynamic/ThirdPerson/Blueprints/BP_GameMode` (`GameplayStatics.GetGameMode`)))
  (`self.OnEnemyDeafeated` _asbp_game_mode))

(event `self.ReceiveBeginPlay`
  (`KismetSystemLibrary.K2_SetTimerDelegate` (delegate `TryToSpawn`) 2.0 true))

(event `TryToSpawn`
  (`self.SpawnFunction`))

(event `SpawnEnemy`
  ;[1 1 1] old code keeping for reference
)

(event `EnemyDeath`
  ;[1 1 1] old code keeping for reference
)

(fn `AddEnemyToQueue`
  (params (EnemyClass :type "/Game/Dynamic/AI/BP_AI Class Reference (by ref)"))
  (`KismetArrayLibrary.Array_Add` (`self.Enemy Queue`) EnemyClass)
  (if (not (`KismetArrayLibrary.Array_IsValidIndex` (`PrimitiveComponent.GetOverlappingActors` (`self.Sphere`) "/Game/Dynamic/AI/BP_AI.BP_AI_C")))
    (`self.SpawnFunction`)))

(fn `SpawnFunction`
  (returns (Success :type Boolean))
  (if (`KismetArrayLibrary.Array_IsValidIndex` (`self.Enemy Queue`))
    (bind _returnvalue (`|SpawnActorFromClass` (`|GetArrayItem` (`self.Enemy Queue`)) (`self.GetTransform`) "Undefined" "MultiplyWithRoot" null null))
    (add `self.OnDestroyed` _returnvalue (`|CreateDelegate` :!event `OnEnemyDeafeated`))
    (`KismetArrayLibrary.Array_Remove` (`self.Enemy Queue`))
    (return true)
    (else
      (return false))))

(fn `UserConstructionScript`)